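; BP_NDI_Receiver is an actor that receives an NDI stream and moves itself using transform data in the stream's metadata.
; The construction script lists available source names; BeginPlay finds the named source and starts the receiver, printing status.
; Each Tick parses the current metadata as XML and applies it to the root's world transform.
; ReadMeta remaps axes, flips signs and scales translation by 100 for Unreal coordinates.
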(event EventBeginPlay
  (bind (_connectioninformation _returnvalue) (Class|NDIIOLibrary|FindNetworkSourcebyName (Variables|Default|GetNDI%20Source%20Name)))
  (if _returnvalue
    (Development|PrintString "Found it!" true true "(R=0.000000,G=1.000000,B=0.000000,A=1.000000)" 1e+01)
    (bind _returnvalue_2 (Class|NDIReceiverComponent|StartReceiver (Variables|Default|GetNDIReceiver) _connectioninformation))
    (Development|PrintString (Utilities|String|ToString(Boolean) _returnvalue_2))
    (else
      (Development|PrintString (Utilities|String|Append (Class|KismetSystemLibrary|GetPathName self) "  no source can be find!") true true "(R=1.000000,G=0.000000,B=0.000000,A=1.000000)" 1e+01))))

(event Collision|EventActorBeginOverlap
  (params (OtherActor :type Actor%20Object%20Reference)))

(event EventTick
  (params (DeltaSeconds :type Float%20%28single-precision%29))
  (bind _ndireceiver (Variables|Default|GetNDIReceiver))
  (bind _returnvalue (Class|NDIReceiverComponent|GetCurrentMetadata _ndireceiver))
  (if (stale EventBeginPlay _returnvalue)
    (Development|PrintString _returnvalue true false)
    (bind (_errormessage _returnvalue_2) (Class|EasyXMLParseManager|LoadfromString _returnvalue)
      (:Successed
        (bind _transform (CallFunction|ReadMeta _returnvalue_2))
        (Transformation|SetWorldTransform (Variables|Default|GetDefaultSceneRoot) _transform false false))
      (:Failed
        (Development|PrintString _errormessage true true "(R=1.000000,G=0.000000,B=0.000000,A=1.000000)" 1e+01)))))

(fn ConstructionScript
  (bind _ndi_sources (Variables|Default|GetNDI%20sources))
  (Utilities|Array|Clear _ndi_sources)
  (for _array_element (Class|NDIIOLibrary|GetNDISourceCollection)
    (Utilities|Array|Add _ndi_sources (.SourceName (Utilities|Struct|BreakNDIConnectionInformation _array_element)))))

(fn ReadMeta
  (params (XML :type Easy%20XML%20Element%20Object%20Reference))
  (return (Math|Transform|MakeTransform (* (Math|Vector|MakeVector (* (Class|EasyXMLElement|ReadFloat XML "tz" 0.0) -1.0) (Class|EasyXMLElement|ReadFloat XML "tx" 0.0) (Class|EasyXMLElement|ReadFloat XML "ty" 0.0)) 1e+02) (Math|Rotator|MakeRotator (* (Class|EasyXMLElement|ReadFloat XML "rz" 0.0) -1.0) (Class|EasyXMLElement|ReadFloat XML "rx" 0.0) (* (Class|EasyXMLElement|ReadFloat XML "ry" 0.0) -1.0)) (Math|Vector|MakeVector (Class|EasyXMLElement|ReadFloat XML "sz" 0.0) (Class|EasyXMLElement|ReadFloat XML "sx" 0.0) (Class|EasyXMLElement|ReadFloat XML "sy" 0.0)))))